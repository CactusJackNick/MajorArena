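; BP_CharacterBase is the third-person player archer, with camera-relative movement, directional dodge rolls, timer-drained sprint stamina and HUD creation.
; Aiming lerps the camera to a shoulder position via timeline, shows a crosshair and drives ACArrowMechanics to spawn and fire arrows.
; E launches cooldown-gated triple homing arrows at nearby BP_AI, tracked by the action bar.
; BP_AI overlaps deal damage unless rolling; death fades out and reloads the level.
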(event `self.ReceiveBeginPlay`
  ;[0.974 1 0] BeginPlay Logic
  (`self.EnableInput` (`GameplayStatics.GetPlayerController` 0))
  (set `self.Health` (`self.MaxHealth`))
  (bind _returnvalue (`|CreateWidget` "/Game/Widgets/HUD_Widget.HUD_Widget_C" (cast `PlayerController` (`self.GetController`) :!pure true)))
  (set `self.widget` _returnvalue)
  (`UserWidget.AddToViewport` _returnvalue 0)
  (set `/Game/Widgets/Health_Widget.CharacterReference` self (`/Game/Widgets/HUD_Widget.Health_Widget` _returnvalue))
  (`PlayerCameraManager.StartCameraFade` :`self` (`GameplayStatics.GetPlayerCameraManager` 0) :`FromAlpha` 1.0 :`Duration` 2.0)
  (bind _asmajor_player_controller (cast `MajorPlayerController` (`self.GetController`)))
  (set `self.CharacterController` _asmajor_player_controller))

(event `InputAxis|MoveForward`
  (params (AxisValue :type "Float (single-precision)"))
  (bind _charactermovement (`self.CharacterMovement`))
  ;[1 0.2389 0.2688] Movement
  (`self.AddMovementInput` (`KismetMathLibrary.GetForwardVector` (`KismetMathLibrary.MakeRotator` 0.0 0.0 (.yaw (`PlayerCameraManager.GetCameraRotation` (`GameplayStatics.GetPlayerCameraManager` 0))))) AxisValue)
  ;[1 0.4654 0.4256] Orient On/Off
  (if (> (`KismetMathLibrary.VSize` (`KismetMathLibrary.MakeVector` AxisValue (stale `InputAxis|MoveRight` AxisValue))) 0.0) :!label _label
    (set `CharacterMovementComponent.bOrientRotationToMovement` false _charactermovement)
    (set `CharacterMovementComponent.bUseControllerDesiredRotation` true _charactermovement)
    (elif (not (`self.isAiming?`))
      (set `CharacterMovementComponent.bOrientRotationToMovement` true _charactermovement)
      (set `CharacterMovementComponent.bUseControllerDesiredRotation` false _charactermovement))))

(event `Key|LeftControl`
  (params (Key :type "Key Structure"))
  ;[1 0 0.01929] DodgeRoll
  (:`Pressed`
    (`self.DodgeRoll` "/Game/Characters/Archer/Animations/DodgeRoll/DodgeRoll_Montage.DodgeRoll_Montage" "W"
      (:`false`
        (`self.DodgeRoll` "/Game/Characters/Archer/Animations/DodgeRoll/Dodge_Back_Montage.Dodge_Back_Montage" "S"
          (:`false`
            (`self.DodgeRoll` "/Game/Characters/Archer/Animations/DodgeRoll/Dodge_LeftMontage.Dodge_LeftMontage" "A"
              (:`false`
                (`self.DodgeRoll` "/Game/Characters/Archer/Animations/DodgeRoll/Dodge_RightMontage.Dodge_RightMontage" "D")))))))))

(event `InputAxis|MoveRight`
  (params (AxisValue :type "Float (single-precision)"))
  ;[1 0.2389 0.2688] Movement
  (`self.AddMovementInput` (`KismetMathLibrary.GetRightVector` (`KismetMathLibrary.MakeRotator` 0.0 0.0 (.yaw (`PlayerCameraManager.GetCameraRotation` (`GameplayStatics.GetPlayerCameraManager` 0))))) AxisValue)
  (goto _label))

(event `InputAction|Aim`
  (params (Key :type "Key Structure"))
  (bind _charactermovement (`self.CharacterMovement`))
  (bind _charactermovement_2 (`self.CharacterMovement`))
  ;[1 0.01949 0] Aiming / Camera for aiming
  (:`Pressed`
    (set `self.isAiming?` true)
    (`/Game/Blueprints/AC_ArrowMechanics.SpawnArrow` (`self.AC_ArrowMechanics`))
    (set `CharacterMovementComponent.bOrientRotationToMovement` false _charactermovement)
    (set `CharacterMovementComponent.bUseControllerDesiredRotation` true _charactermovement)
    (bind _returnvalue (`|CreateWidget` "/Game/Widgets/Bow_Crosshair.Bow_Crosshair_C"))
    (bind _output_get (set `self.BowCrosshairWidget` _returnvalue))
    (`UserWidget.AddToViewport` _output_get 0)
    (bind (_direction _zoomin) (`Timeline|ZoomIn` :`NewTime` 1.0 :!label _label_2)
      (:`Update`
        (bind _returnvalue_2 (`KismetMathLibrary.VLerp` (`SceneComponent.RelativeLocation` (`self.Chase`)) (`SceneComponent.RelativeLocation` (`self.Shoulder`)) _zoomin))
        (`SceneComponent.K2_SetRelativeLocation` (`self.Camera`) _returnvalue_2 false false))
      (:`Finished`
        (`SceneComponent.K2_SetRelativeLocation` (`self.Camera`) _returnvalue_2 false false))))
  (:`Released`
    (set `self.isAiming?` false)
    (`/Game/Blueprints/AC_ArrowMechanics.DestroyArrow` (`self.AC_ArrowMechanics`))
    (set `CharacterMovementComponent.bOrientRotationToMovement` true _charactermovement_2)
    (set `CharacterMovementComponent.bUseControllerDesiredRotation` false _charactermovement_2)
    (`KismetSystemLibrary.Delay` 0.2)
    (bind _bowcrosshairwidget (`self.BowCrosshairWidget`)
      (:`then`
        (`Widget.RemoveFromParent` _bowcrosshairwidget)
        (set `self.BowCrosshairWidget` null)
        (goto _label_2 :!via `Reverse`))
      (:`else`))))

(event `ShootArrow`
  ;[1 1 1] Traceline Arrow and then destroy it (Not IN USE)
)

(event `InputAction|ShootArrow`
  (params (Key :type "Key Structure"))
  ;[1 0.01752 0] Shoot arrow with LMB only while Aiming
  (:`Pressed`
    (if (not (`self.isAiming?`))
      (set `self.isShooting?` false)
      (else
        (set `self.isShooting?` true)
        (`KismetSystemLibrary.Delay` 0.2)
        (`/Game/Blueprints/AC_ArrowMechanics.FireArrowBegin` (`self.AC_ArrowMechanics`))
        (`/Game/Blueprints/AC_ArrowMechanics.SpawnArrow` (`self.AC_ArrowMechanics`))))))

(event `Check Aim`
  ;[0.04076 0.9602 1] Remove crosshair in case of fast input
  (if (not (`self.isAiming?`))
    (`/Game/Blueprints/AC_ArrowMechanics.DestroyArrow` (`self.AC_ArrowMechanics`))
    (bind _output_get (set `self.BowCrosshairWidget` (`self.BowCrosshairWidget`)))
    (`Widget.SetVisibility` _output_get "Hidden")))

(event `self.ReceiveAnyDamage`
  (params (Damage :type "Float (single-precision)") (DamageType :type "DamageType Object Reference") (InstigatedBy :type "Controller Object Reference") (DamageCauser :type "Actor Object Reference"))
  (`GameplayStatics.PlaySoundAtLocation` "/Game/Sounds/hitReactSound.hitReactSound" (0.0 0.0 0.0) (struct) 1.0 1.0 0.0 null null null null)
  (`self.PlayAnimMontage` "/Game/Characters/Archer/Animations/HitReact_Large_From_Front_Montage.HitReact_Large_From_Front_Montage"))

(event `self.CapsuleComponent.OnComponentBeginOverlap`
  (params (OverlappedComponent :type "PrimitiveComponent Object Reference") (OtherActor :type "Actor Object Reference") (OtherComp :type "PrimitiveComponent Object Reference") (OtherBodyIndex :type Integer) (bFromSweep :type Boolean) (SweepResult :type "HitResult Structure (by ref)"))
  ;[0.2546 0.5897 1] AI damage to Player & If player is rolling apply 0 damage
  (if (`self.isRolling?`)
    (bind _returnvalue (`GameplayStatics.ApplyDamage` null))
    (`self.EditHealth` _returnvalue)
    (else
      (bind _asbp_ai (cast `/Game/AI/BP_AI` OtherActor))
      (bind _returnvalue_2 (`GameplayStatics.ApplyDamage` self (`/Game/AI/BP_AI.AIDamage` _asbp_ai) null _asbp_ai))
      (`self.EditHealth` _returnvalue_2)
      (if (<= (`self.Health`) 0.0)
        (`self.Die`)
        (`PrimitiveComponent.SetCollisionEnabled` (`self.CapsuleComponent`) "NoCollision")))))

(event `Die`
  ;[1 0.7171 0.2353] Death And Respawn Level by name
  (`self.DisableInput` null)
  (`SkeletalMeshComponent.PlayAnimation` (`self.Mesh`) "/Game/Characters/Archer/Animations/Standing_Death.Standing_Death" false)
  (`PlayerCameraManager.StartCameraFade` :`self` (`GameplayStatics.GetPlayerCameraManager` 0) :`ToAlpha` 1.0 :`Duration` 5.0)
  (`KismetSystemLibrary.Delay` 4.8)
  (bind _returnvalue (`GameplayStatics.GetCurrentLevelName` true))
  (`GameplayStatics.OpenLevel` (`KismetStringLibrary.Conv_StringToName` _returnvalue)))

(event `InputAction|Sprint` :consume false
  (params (Key :type "Key Structure"))
  (bind _charactermovement (`self.CharacterMovement`))
  (bind _charactercontroller (`self.CharacterController`))
  ;[0.005386 0.2329 1] Stamina Logic
  (:`Pressed`
    (`MajorPlayerController.RequestSprintStart` _charactercontroller)
    (set `self.Can Sprint` true)
    (if (`self.Can Sprint`)
      (set `CharacterMovementComponent.MaxWalkSpeed` 900.0 _charactermovement)
      (bind _returnvalue (`KismetSystemLibrary.K2_SetTimerDelegate` (delegate `DrainStamina`) 0.1 true))
      (set `self.timer Loop` _returnvalue)))
  (:`Released`
    (`MajorPlayerController.RequestSprintEnd` _charactercontroller)
    (set `CharacterMovementComponent.MaxWalkSpeed` 600.0 _charactermovement)
    (`KismetSystemLibrary.K2_ClearAndInvalidateTimerHandle` (`self.timer Loop`))
    (set `self.Can Sprint` false)))

(event `EditHealth`
  (params (Amount :type "Float (double-precision)"))
  ;[0.1565 1 0.1194] Clamp Health Value
  (set `self.Health` (`KismetMathLibrary.FClamp` (+ Amount (`self.Health`)) 0.0 (`self.MaxHealth`))))

(event `DrainStamina`
  (bind _staminabar (`/Game/Widgets/HUD_Widget.StaminaBar` (`self.widget`)))
  ;[0.005386 0.2329 1] Stamina Logic
  (if (`self.Can Sprint`)
    (`/Game/Widgets/StaminaBar.DecreaseStamina` _staminabar 2.0)
    (if (<= (`/Game/Widgets/StaminaBar.GetStamina` _staminabar) 0.0)
      (set `self.Can Sprint` false)
      (`MajorPlayerController.RequestSprintEnd` (`self.CharacterController`))
      (else
        (set `self.Can Sprint` true)))
    (else
      (set `CharacterMovementComponent.MaxWalkSpeed` 600.0 (`self.CharacterMovement`)))))

(event `self.ReceiveTick`
  (params (DeltaSeconds :type "Float (single-precision)"))
  ;[0.004949 0.2185 1] Increase stamina while standing
  (if (<= (`KismetMathLibrary.VSize` (`self.GetVelocity`)) 0.0)
    (`KismetSystemLibrary.Delay` 0.2)
    (`/Game/Widgets/StaminaBar.IncreaseStamina` (`/Game/Widgets/HUD_Widget.StaminaBar` (`self.widget`)) 2.0)))

(event `FireHomingTripleArrow`
  (bind _returnvalue (`GameplayStatics.GetPlayerCharacter` 0))
  (bind (_yaw _pitch) (`KismetMathLibrary.GetYawPitchFromVector` (`self.GetActorForwardVector`)))
  (bind (_yaw_2 _pitch_2) (`KismetMathLibrary.GetYawPitchFromVector` (`self.GetActorForwardVector`)))
  (bind _actionbarslot_ui (`/Game/Widgets/HUD_Widget.ActionBarSlot_UI` (`self.widget`)))
  (bind (_yaw_3 _pitch_3) (`KismetMathLibrary.GetYawPitchFromVector` (`self.GetActorForwardVector` _returnvalue)))
  (bind _returnvalue_2 (`SceneComponent.GetSocketLocation` (`Character.Mesh` _returnvalue) "arrow_socket"))
  (bind _cooldownduration (`/Game/Widgets/ActionBarSlot_UI.CooldownDuration` _actionbarslot_ui))
  (if (not (`self.IsOnCooldown`))
    (bind _outactors (`GameplayStatics.GetAllActorsOfClass` "/Game/AI/BP_AI.BP_AI_C"))
    (for _array_element _outactors
      (bind _returnvalue_3 (`self.GetDistanceTo` _array_element))
      (if (< _returnvalue_3 (`self.NearestDistance`))
        (bind _output_get (set `self.NearestEnemy` _array_element))
        (set `self.NearestDistance` _returnvalue_3)
        (bind _mesh (`Character.Mesh` (cast `/Game/AI/BP_AI` _output_get :!pure true)))
        (`|SpawnActorFromClass` "/Game/Blueprints/BP_WhiteArrow.BP_WhiteArrow_C" (`KismetMathLibrary.MakeTransform` _returnvalue_2 (`KismetMathLibrary.MakeRotator` 0.0 (+ _pitch 15.0) (+ _yaw 15.0))) "Undefined" "MultiplyWithRoot" null _mesh null)
        (`|SpawnActorFromClass` "/Game/Blueprints/BP_WhiteArrow.BP_WhiteArrow_C" (`KismetMathLibrary.MakeTransform` _returnvalue_2 (`KismetMathLibrary.MakeRotator` 0.0 (+ _pitch_3 15.0) (+ _yaw_3 2.0))) "Undefined" "MultiplyWithRoot" null _mesh null)
        (`|SpawnActorFromClass` "/Game/Blueprints/BP_WhiteArrow.BP_WhiteArrow_C" (`KismetMathLibrary.MakeTransform` _returnvalue_2 (`KismetMathLibrary.MakeRotator` 0.0 (+ _pitch_2 15.0) (- _yaw_2 15.0))) "Undefined" "MultiplyWithRoot" null _mesh null)
        (set `self.IsOnCooldown` true)
        (`/Game/Widgets/ActionBarSlot_UI.StartCooldown` _actionbarslot_ui _cooldownduration)
        (`|PlayMontage` (`self.Mesh`) "/Game/Characters/Archer/Animations/Aim/Shoot.Shoot"
          (:`then`
            (`KismetSystemLibrary.K2_SetTimer` null "ResetCooldown" _cooldownduration)))))))

(event `ResetCooldown`
  (set `self.IsOnCooldown` false)
  (set `self.NearestDistance` 99999.0))

(event `Key|E`
  (params (Key :type "Key Structure"))
  (:`Pressed`
    (`self.FireHomingTripleArrow`)
    (if (== (`/Game/Widgets/ActionBarSlot_UI.CooldownDuration` (`/Game/Widgets/HUD_Widget.ActionBarSlot_UI` (`self.widget`))) 0.0)
      (set `self.IsOnCooldown` false)
      (`KismetSystemLibrary.K2_ClearTimer` null "ResetCooldown"))))

(fn `GetHealth`
  (returns (Result :type "Float (double-precision)"))
  (return (`self.Health`)))

(fn `GetHealthAsRatio`
  (returns (Result :type "Float (double-precision)"))
  (bind _result (`self.GetHealth`))
  (return (/ _result (`self.MaxHealth`))))

(fn `UserConstructionScript`)