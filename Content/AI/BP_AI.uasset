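; Enemy AI character with health, an overhead-style health widget and a three-stage melee combo.
; Arrow overlaps apply ArrowDamage through clamped health, and at zero the enemy plays a dying animation and is destroyed.
; Attack, apparently behavior-tree driven, starts DoOnce-gated montages that toggle TriggerHealth collision, with saved attacks continuing the combo.
; Overlapping a dead player character stops attacks; a DodgeRoll macro polls player input.
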(event `self.ReceiveBeginPlay`
  ;[1 1 1] Creating Health Widget
  (set `self.Health` (`self.MaxHealth`))
  (bind _ashealth_widget (cast `/Game/Widgets/Health_Widget` (`WidgetComponent.GetWidget` (`self.HealthWidget`))))
  (set `/Game/Widgets/Health_Widget.CharacterReference` self _ashealth_widget)
  (`PrimitiveComponent.SetCollisionEnabled` (`self.Trigger_Health`) "NoCollision"))

(event `EditHealth`
  (params (Amount :type "Float (double-precision)"))
  ;[1 1 1] Setting Health
  (set `self.Health` (`KismetMathLibrary.FClamp` (+ Amount (`self.Health`)) 0.0 (`self.MaxHealth`))))

(event `self.CapsuleComponent.OnComponentBeginOverlap`
  (params (OverlappedComponent :type "PrimitiveComponent Object Reference") (OtherActor :type "Actor Object Reference") (OtherComp :type "PrimitiveComponent Object Reference") (OtherBodyIndex :type Integer) (bFromSweep :type Boolean) (SweepResult :type "HitResult Structure (by ref)"))
  ;[0.1527 1 0.3434] Damage Enemy / Decrease Health
  (`|ExecutionSequence`
    (:`then_0`
      (bind _asbp_arrow (cast `/Game/Blueprints/BP_Arrow` OtherActor))
      (`self.EditHealth` (`/Game/Blueprints/BP_Arrow.arrowDamage` _asbp_arrow))
      (`self.K2_DestroyActor` _asbp_arrow)
      (if (<= (`self.Health`) 0.0)
        (`self.SetActorEnableCollision` false)
        ;[0.08121 1 0.1267] Disable input/ Play death animation
        (`CharacterMovementComponent.SetMovementMode` (`self.CharacterMovement`) "MOVE_None" 0)
        (`SceneComponent.SetVisibility` (`self.HealthWidget`) false false)
        (`SkeletalMeshComponent.PlayAnimation` (`self.Mesh`) "/Game/AI/MutantAnimations/Mutant_Dying.Mutant_Dying" false)
        (`KismetSystemLibrary.Delay` 5.0)
        (`self.K2_DestroyActor`)))
    (:`then_1`
      (bind _asbp_character_base (cast `/Game/Characters/BP_CharacterBase` OtherActor))
      (bind _result (`/Game/Characters/BP_CharacterBase.GetHealth` _asbp_character_base))
      (if (<= _result 0.0)
        (`self.Stop Combo`)
        (set `self.can Attack?` false)))))

(event `Melee AttackComboFromBT`
  ;[0.09375 0.09375 0.09375] Basic attack System
  ;;[1 0.195 0.335] Attack Input
  (if (`self.can Attack?`)
    (`self.melee attack`)))

(event `Attack1`
  ;[0.09375 0.09375 0.09375] Basic attack System
  ;;[1 1 1] Attack1
  (`/Engine/EditorBlueprintResources/StandardMacros.DoOnce` false :!label _label
    (:`Completed`
      (`KismetSystemLibrary.Delay` 0.2)
      (`PrimitiveComponent.SetCollisionEnabled` (`self.Trigger_Health`) "QueryAndPhysics")
      (`|PlayMontage` (`self.Mesh`) "/Game/AI/MutantAnimations/Combo1_Montage.Combo1_Montage"
        (:`then`
          (`PrimitiveComponent.SetCollisionEnabled` (`self.Trigger_Health`) "NoCollision")
          (set `self.attackIndex` 1)
          (goto _label :!via `Reset`))))))

(event `melee attack`
  ;[0.09375 0.09375 0.09375] Basic attack System
  ;;[1 0.4157 0.5259] Melee Attack
  (if (`self.isAttacking?`)
    (set `self.saveAttack?` true)
    (else
      (set `self.isAttacking?` true)
      (switch `int` (`self.attackIndex`) :!label _label_2
        (:`0`
          (`self.Attack1`))
        (:`1`
          (`self.Attack2`))
        (:`2`
          (`self.Attack3`))))))

(event `Attack2`
  ;[0.09375 0.09375 0.09375] Basic attack System
  ;;[1 1 1] Attack2
  (`/Engine/EditorBlueprintResources/StandardMacros.DoOnce` false :!label _label_3
    (:`Completed`
      (`KismetSystemLibrary.Delay` 1.3)
      (`PrimitiveComponent.SetCollisionEnabled` (`self.Trigger_Health`) "QueryAndPhysics")
      (`|PlayMontage` (`self.Mesh`) "/Game/AI/MutantAnimations/Combo2_Montage.Combo2_Montage"
        (:`then`
          (`PrimitiveComponent.SetCollisionEnabled` (`self.Trigger_Health`) "NoCollision")
          (set `self.attackIndex` 2)
          (goto _label_3 :!via `Reset`))))))

(event `MeleeAttackCombo`
  ;[0.09375 0.09375 0.09375] Basic attack System
  ;;[1 0.3112 0.3511] Combo Continue
  (if (`self.saveAttack?`)
    (set `self.saveAttack?` false)
    (goto _label_2)
    (else
      (`self.Stop Combo`))))

(event `Attack3`
  ;[0.09375 0.09375 0.09375] Basic attack System
  ;;[1 1 1] Attack3
  (`/Engine/EditorBlueprintResources/StandardMacros.DoOnce` false :!label _label_4
    (:`Completed`
      (`KismetSystemLibrary.Delay` 0.7)
      (`PrimitiveComponent.SetCollisionEnabled` (`self.Trigger_Health`) "QueryAndPhysics")
      (`|PlayMontage` (`self.Mesh`) "/Game/AI/MutantAnimations/Combo3_Montage.Combo3_Montage"
        (:`then`
          (set `self.attackIndex` 3)
          (`PrimitiveComponent.SetCollisionEnabled` (`self.Trigger_Health`) "NoCollision")
          (goto _label_4 :!via `Reset`))))))

(event `Stop Combo`
  ;[0.09375 0.09375 0.09375] Basic attack System
  ;;[1 0.3695 0.4493] Stop Combo / Attack
  (set `self.isAttacking?` false)
  (set `self.attackIndex` 0))

(fn `Attack`
  (returns (AnimationDuration :type "Float (double-precision)"))
  (`self.Melee AttackComboFromBT`)
  (return 0.4))

(fn `GetHealth`
  (returns (Result :type "Float (double-precision)"))
  (return (`self.Health`)))

(fn `GetHealthAsRatio`
  (returns (Result :type "Float (double-precision)"))
  (bind _result (`self.GetHealth`))
  (return (/ _result (`self.MaxHealth`))))

(fn `UserConstructionScript`)