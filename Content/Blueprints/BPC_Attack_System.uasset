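; Actor component that runs a three-hit melee combo on its BP_CharacterBase owner from the IA_Attack input.
; AttackIndex selects which combo montage plays; each DoOnce-guarded attack waits briefly, starts its montage and advances the index.
; Input during IsAttacking buffers SaveAttack, which MeleeAttackCombo consumes to chain the next hit, otherwise calling StopCombo to reset.
; Nothing here sets IsAttacking true or calls MeleeAttackCombo.
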(event `self.ReceiveBeginPlay`
  (bind _asbp_character_base (cast `/Game/Characters/BP_CharacterBase` (`self.GetOwner`)))
  (set `self.Character Mesh` (`Character.Mesh` _asbp_character_base)))

(event `EnhancedInput|/Game/Blueprints/IA_Attack`
  (params (ActionValue :type Boolean) (ElapsedSeconds :type "Float (double-precision)") (TriggeredSeconds :type "Float (double-precision)") (InputAction :type "InputAction Object Reference" :default "/Game/Blueprints/IA_Attack.IA_Attack"))
  ;[0.09375 0.09375 0.09375] Basic attack System
  ;;[1 0.195 0.335] Attack Input
  (:`Started`
    (if (`self.can Attack?`)
      (`self.melee attack`))))

(event `Attack1`
  ;[0.09375 0.09375 0.09375] Basic attack System
  ;;[1 1 1] Attack1
  (`/Engine/EditorBlueprintResources/StandardMacros.DoOnce` false :!label _label
    (:`Completed`
      (`KismetSystemLibrary.Delay` 0.1)
      (`|PlayMontage` (`self.Character Mesh`) "/Game/AI/MutantAnimations/Combo1_Montage.Combo1_Montage"
        (:`then`
          (set `self.attackIndex` 1)
          (goto _label :!via `Reset`))))))

(event `melee attack`
  ;[0.09375 0.09375 0.09375] Basic attack System
  ;;[1 0.4157 0.5259] Melee Attack
  (if (`self.isAttacking?`)
    (set `self.saveAttack?` true)
    (else
      (set `self.saveAttack?` false)
      (switch `int` (`self.attackIndex`) :!label _label_2
        (:`0`
          (`self.Attack1`))
        (:`1`
          (`self.Attack2`))
        (:`2`
          (`self.Attack3`))))))

(event `Attack2`
  ;[0.09375 0.09375 0.09375] Basic attack System
  ;;[1 1 1] Attack2
  (`/Engine/EditorBlueprintResources/StandardMacros.DoOnce` false :!label _label_3
    (:`Completed`
      (`KismetSystemLibrary.Delay` 0.1)
      (`|PlayMontage` (`self.Character Mesh`) "/Game/AI/MutantAnimations/Combo2_Montage.Combo2_Montage"
        (:`then`
          (set `self.attackIndex` 2)
          (goto _label_3 :!via `Reset`))))))

(event `MeleeAttackCombo`
  ;[0.09375 0.09375 0.09375] Basic attack System
  ;;[1 0.3112 0.3511] Combo Continue
  (if (`self.saveAttack?`)
    (set `self.saveAttack?` false)
    (goto _label_2)
    (else
      (`self.Stop Combo`))))

(event `Attack3`
  ;[0.09375 0.09375 0.09375] Basic attack System
  ;;[1 1 1] Attack3
  (`/Engine/EditorBlueprintResources/StandardMacros.DoOnce` false :!label _label_4
    (:`Completed`
      (`KismetSystemLibrary.Delay` 0.1)
      (`|PlayMontage` (`self.Character Mesh`) "/Game/AI/MutantAnimations/Combo3_Montage.Combo3_Montage"
        (:`then`
          (set `self.attackIndex` 3)
          (goto _label_4 :!via `Reset`))))))

(event `Stop Combo`
  ;[0.09375 0.09375 0.09375] Basic attack System
  ;;[1 0.3695 0.4493] Stop Combo / Attack
  (set `self.isAttacking?` false)
  (set `self.attackIndex` 0))